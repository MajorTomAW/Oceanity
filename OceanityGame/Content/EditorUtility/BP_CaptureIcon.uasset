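; BP_CaptureIcon is an editor utility that renders static meshes into icon textures.
; LoadMesh applies the selected mesh, and Engine and Turret events apply preset transforms to frame it for the shot.
; CaptureIcon captures the scene with a SceneCapture2D, then saves the render target as a static texture named after the mesh in the Captured icons folder.
; If that texture already exists, it deletes it and calls itself again to recapture.
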(event `Engine`
  (`SceneComponent.K2_SetRelativeTransform` (`self.StaticMesh`) (`KismetMathLibrary.MakeTransform` (74.137885 0.321432 -7.304563) (struct :`Yaw` 136.400001) (0.3 0.3 0.3)) false false))

(event `Turret`
  (`SceneComponent.K2_SetRelativeTransform` (`self.StaticMesh`) (`KismetMathLibrary.MakeTransform` (89.033959 0.321432 -7.304563) (struct :`Yaw` 136.400001) (0.3 0.3 0.3)) false false))

(event `LoadMesh`
  (`StaticMeshComponent.SetStaticMesh` (`self.StaticMesh`) (`self.SelectedMesh`)))

(event `CaptureIcon`
  (bind _capturecomponent2d (`SceneCapture2D.CaptureComponent2D` (`self.CaptureActor`)))
  (set `self.ObjectPath` (`KismetStringLibrary.Concat_StrStr` "/Game/Textures/Icons/Captured/" (`KismetStringLibrary.Concat_StrStr` "T_" (`KismetStringLibrary.Replace` (`KismetSystemLibrary.GetDisplayName` (`StaticMeshComponent.StaticMesh` (`self.StaticMesh`))) "SM_"))))
  (`SceneCaptureComponent2D.CaptureScene` _capturecomponent2d)
  (bind _returnvalue (`EditorAssetLibrary.DoesAssetExist` (`self.ObjectPath`)))
  (if _returnvalue
    (`EditorAssetLibrary.DeleteAsset` (`self.ObjectPath`))
    (`self.CaptureIcon`)
    (else
      (bind _returnvalue_2 (`KismetRenderingLibrary.RenderTargetCreateStaticTexture2DEditorOnly` (`SceneCaptureComponent2D.TextureTarget` _capturecomponent2d) (`self.ObjectPath`) "TC_EditorIcon"))
      (bind _output_get (set `self.GeneratedTextureTarget` _returnvalue_2))
      (`EditorAssetLibrary.SaveLoadedAsset` _output_get))))

(fn `UserConstructionScript`)