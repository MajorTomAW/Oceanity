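; Player-controlled ship character that moves by physics forces on its capsule, with mouse cursor hidden and Enhanced Input set up at BeginPlay.
; Look input drives controller yaw and pitch, while move input feeds sMove, which pushes forward or back at Left and Right points, harder near standstill.
; Steering adds forward force on one side as differential thrust; all thrust, steering included, stops at a speed cap.
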(event `Key|P`
  (params (Key :type "Key Structure")))

(event `self.ReceiveBeginPlay`
  (bind _asplayer_controller (cast `PlayerController` (`self.GetController`)))
  (message `EnhancedInputSubsystemInterface.AddMappingContext` (pcsubsystem `EnhancedInputLocalPlayerSubsystem` _asplayer_controller) "/Game/EnhancedInput/IMC_PlayerInput.IMC_PlayerInput" 0 (struct))
  (`WidgetBlueprintLibrary.SetInputMode_GameOnly` _asplayer_controller)
  (set `PlayerController.bShowMouseCursor` false _asplayer_controller))

(event `EnhancedInput|/Game/EnhancedInput/InputActions/IA_Look`
  (params (ActionValue :type "Vector2D Structure") (ElapsedSeconds :type "Float (double-precision)") (TriggeredSeconds :type "Float (double-precision)") (InputAction :type "InputAction Object Reference" :default "/Game/EnhancedInput/InputActions/IA_Look.IA_Look"))
  (bind (_x _y) (`KismetMathLibrary.BreakVector2D` ActionValue))
  (:`Triggered`
    (`self.AddControllerYawInput` _x)
    (`self.AddControllerPitchInput` _y)))

(event `EnhancedInput|/Game/EnhancedInput/InputActions/IA_Move`
  (params (ActionValue :type "Vector2D Structure") (ElapsedSeconds :type "Float (double-precision)") (TriggeredSeconds :type "Float (double-precision)") (InputAction :type "InputAction Object Reference" :default "/Game/EnhancedInput/InputActions/IA_Move.IA_Move"))
  (:`Triggered`
    (`self.sMove` ActionValue)))

(event `sMove`
  (params (Value :type "Vector2D Structure"))
  (bind (_x _y) (`KismetMathLibrary.BreakVector2D` Value))
  (bind _returnvalue (`KismetMathLibrary.VSize` (`self.GetVelocity`)))
  (bind _returnvalue_2 (* (`self.GetActorForwardVector`) (* (`KismetMathLibrary.SelectFloat` 3.0 1.5 (`KismetMathLibrary.InRange_FloatFloat` _returnvalue -10.0 10.0)) 600000.0) _y (* (`GameplayStatics.GetWorldDeltaSeconds`) 100.0)))
  (if (< _returnvalue 800.0)
    (`PrimitiveComponent.AddForceAtLocation` (`self.CapsuleComponent`) _returnvalue_2 (`SceneComponent.K2_GetComponentLocation` (`self.left`)) "None")
    (`PrimitiveComponent.AddForceAtLocation` (`self.CapsuleComponent`) _returnvalue_2 (`SceneComponent.K2_GetComponentLocation` (`self.right`)) "None")
    (if (!= _x 0.0)
      (`PrimitiveComponent.AddForceAtLocation` (`self.CapsuleComponent`) (* (`self.GetActorForwardVector`) 200000.0 (* (`GameplayStatics.GetWorldDeltaSeconds`) 100.0)) (`SceneComponent.K2_GetComponentLocation` (select `bool` (== _x 1.0) :`false` (`self.right`) :`true` (`self.left`))) "None"))))

(fn `UserConstructionScript`)