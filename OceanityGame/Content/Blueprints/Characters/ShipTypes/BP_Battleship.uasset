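; Battleship ship-type Blueprint that maps player keys to thrust settings and an upward jump.
; Number keys 1 to 4 call ServerChangeAcceleration, defined outside this file, with rising max acceleration and force, while key 9 passes far higher values.
; Right mouse fires the sJumpy event, which applies a mass-independent upward force to the capsule.
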(event `Key|One`
  (params (Key :type "Key Structure"))
  (:`Pressed`
    (`self.Server_ChangeAcceleration` 800.0 600000.0)))

(event `Key|Two`
  (params (Key :type "Key Structure"))
  (:`Pressed`
    (`self.Server_ChangeAcceleration` 1600.0 900000.0)))

(event `Key|Three`
  (params (Key :type "Key Structure"))
  (:`Pressed`
    (`self.Server_ChangeAcceleration` 2400.0 1200000.0)))

(event `Key|Four`
  (params (Key :type "Key Structure"))
  (:`Pressed`
    (`self.Server_ChangeAcceleration` 3200.0 1600000.0)))

(event `Key|Nine`
  (params (Key :type "Key Structure"))
  (:`Pressed`
    (`self.Server_ChangeAcceleration` 5000000.0 60000000.0)))

(event `Key|RightMouseButton`
  (params (Key :type "Key Structure"))
  (:`Pressed`
    (`self.sJumpy`)))

(event `sJumpy`
  (`PrimitiveComponent.AddForce` (`self.CapsuleComponent`) (0.0 0.0 100000.0) "None" true))

(fn `UserConstructionScript`)