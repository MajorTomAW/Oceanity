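; Enemy AI controller that pilots a BP_BattleShip to chase and shoot at player-controlled battleships.
; Each tick, the target direction's dot with the ship's right vector selects left, right or both engines for physics thrust, with straight thrust speed-capped.
; Within range, it aims the turret and spawns projectiles.
; Delays on Tick throttle firing and periodic retargeting to the nearest ship owned by a PC_GameController.
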(event `self.ReceivePossess`
  (params (PossessedPawn :type "Pawn Object Reference"))
  (bind _asbp_battle_ship (cast `/Game/Blueprints/Characters/ShipTypes/BP_BattleShip` PossessedPawn))
  (set `self.As BP Battle Ship` _asbp_battle_ship)
  (`KismetSystemLibrary.Delay` 2.0)
  (bind _outactors (`GameplayStatics.GetAllActorsOfClass` "/Game/Blueprints/Characters/ShipTypes/BP_BattleShip.BP_BattleShip_C"))
  (for _array_element _outactors
    (if (!= _array_element self)
      (set `self.Target` _array_element))))

(event `self.ReceiveTick`
  (params (DeltaSeconds :type "Float (single-precision)"))
  (bind _as_bp_battle_ship (`self.As BP Battle Ship`))
  (bind _as_bp_battle_ship_2 (`self.As BP Battle Ship`))
  (bind _as_bp_battle_ship_3 (`self.As BP Battle Ship`))
  (bind _returnvalue (`self.K2_GetActorLocation` _as_bp_battle_ship))
  (bind _projectilespawn (`ShipBase.ProjectileSpawn` _as_bp_battle_ship))
  (bind _capsulecomponent (`Character.CapsuleComponent` _as_bp_battle_ship_2))
  (bind _returnvalue_2 (* (`self.GetActorForwardVector` _as_bp_battle_ship_2) 700000.0))
  (bind _target (`self.Target`)
    (:`then`
      (bind _output_get (set `self.TargetLocation` (`self.K2_GetActorLocation` _target)))
      (`|ExecutionSequence`
        (:`then_0`
          (bind _dot (`self.fCalculateForce`))
          (if (`KismetMathLibrary.InRange_FloatFloat` _dot -0.2 0.2)
            (if (< (`KismetMathLibrary.VSize` (`self.GetVelocity` _as_bp_battle_ship_2)) 600.0)
              (`PrimitiveComponent.AddForceAtLocation` _capsulecomponent _returnvalue_2 (`SceneComponent.K2_GetComponentLocation` (`ShipBase.EngineLeft` _as_bp_battle_ship_2)) "None")
              (`PrimitiveComponent.AddForceAtLocation` _capsulecomponent _returnvalue_2 (`SceneComponent.K2_GetComponentLocation` (`ShipBase.EngineRight` _as_bp_battle_ship_2)) "None"))
            (else
              (`PrimitiveComponent.AddForceAtLocation` _capsulecomponent (* (`self.GetActorForwardVector` _as_bp_battle_ship_3) 700000.0) (`SceneComponent.K2_GetComponentLocation` (select `bool` (> _dot 0.0) :`false` (`ShipBase.EngineRight` _as_bp_battle_ship_3) :`true` (`ShipBase.EngineLeft` _as_bp_battle_ship_3))) "None"))))
        (:`then_1`
          (if (< (`KismetMathLibrary.Vector_Distance` _output_get _returnvalue) 5000.0)
            (`SceneComponent.K2_SetWorldRotation` (`ShipBase.TurretBase` _as_bp_battle_ship) (`KismetMathLibrary.FindLookAtRotation` _returnvalue _output_get) false false)
            (`KismetSystemLibrary.Delay` 0.2)
            (`|SpawnActorFromClass` "/Game/Blueprints/Projectiles/BP_BattleshipProjectile.BP_BattleshipProjectile_C" (`KismetMathLibrary.MakeTransform` (`SceneComponent.K2_GetComponentLocation` _projectilespawn) (`SceneComponent.K2_GetComponentRotation` _projectilespawn)) "Undefined" "MultiplyWithRoot" (`self.As BP Battle Ship`) null)))
        (:`then_2`
          (`KismetSystemLibrary.Delay` 2.0)
          (bind _outactors (`GameplayStatics.GetAllActorsOfClass` "/Game/Blueprints/Characters/ShipTypes/BP_BattleShip.BP_BattleShip_C"))
          (for _array_element _outactors
            (if (and (!= _array_element self) (== (`GameplayStatics.GetObjectClass` (`Pawn.GetController` _array_element)) "/Game/Blueprints/GameLogic/Game/PC_GameController.PC_GameController_C"))
              (`KismetArrayLibrary.Array_AddUnique` (`self.PossibleActors`) _array_element)
              (bind _asbp_battle_ship (cast `/Game/Blueprints/Characters/ShipTypes/BP_BattleShip` (`.ReturnValue` (`GameplayStatics.FindNearestActor` (`self.K2_GetActorLocation` (`self.As BP Battle Ship`)) (`self.PossibleActors`)))))
              (set `self.Target` _asbp_battle_ship))))))
    (:`else`)))

(fn `fCalculateForce`
  (returns (Dot :type "Float (double-precision)"))
  (locals (Direction :type "Vector Structure" :default (0.0 0.0 0.0)))
  (return (`KismetMathLibrary.Dot_VectorVector` (`KismetMathLibrary.Normal` (- (`self.K2_GetActorLocation` (`self.Target`)) (`self.K2_GetActorLocation` (`self.As BP Battle Ship`)))) (`self.GetActorRightVector` (`self.As BP Battle Ship`)))))

(fn `UserConstructionScript`)